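; BP_INT_SWITCH is an interactable switch that toggles between on and off when interacted with.
; Interact checks the SwitchOn boolean and calls SwitchedON or SwitchedOFF to flip it.
; Both functions play the same 2D button-press sound, and the construction script only calls its parent.
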(fn `Interact`
  ;[1 1 1] Determines whether the switch is on or off based off of the interact function
  (if (not (`self.SwitchOn`))
    (`self.SwitchedON`)
    (else
      (`self.SwitchedOFF`))))

(fn `SwitchedOFF`
  ;[1 1 1] Switches off a boolean and plays  a sound
  (`GameplayStatics.PlaySound2D` "/Game/MyContent/SoundEffects/Button_Press_Sound_Effect.Button_Press_Sound_Effect" 1.0 1.0 0.0 null null)
  (set `self.SwitchOn` false))

(fn `SwitchedON`
  ;[1 1 1] Switches on a boolean and plays  a sound
  (`GameplayStatics.PlaySound2D` "/Game/MyContent/SoundEffects/Button_Press_Sound_Effect.Button_Press_Sound_Effect" 1.0 1.0 0.0 null null)
  (set `self.SwitchOn` true))

(fn `UserConstructionScript`
  (`parent.UserConstructionScript`))