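; Switch interactable that adds or removes a key on an assigned door.
; Overrides the parent's switched-on and switched-off functions, running the parent logic before calling AddKey or RemoveKey on the Door reference.
; If no valid Door is assigned, it skips both the parent logic and the key change and prints a stuck-door message.
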(fn `SwitchedOFF`
  ;[1 1 1] adds key when switched off and tells you when a door hasnt been assigned
  (`self.Door`
    (:`then`
      (`parent.SwitchedOFF`)
      (`/Game/MyContent/Interactables/BP_DOOR.RemoveKey` (`self.Door`) true))
    (:`else`
      (`KismetSystemLibrary.PrintString` "door STUCK"))))

(fn `SwitchedON`
  ;[1 1 1] adds key when switched on and tells you when a door hasnt been assigned
  (`self.Door`
    (:`then`
      (`parent.SwitchedON`)
      (`/Game/MyContent/Interactables/BP_DOOR.AddKey` (`self.Door`) true))
    (:`else`
      (`KismetSystemLibrary.PrintString` "DOOR STUCK"))))

(fn `UserConstructionScript`
  (`parent.UserConstructionScript`))