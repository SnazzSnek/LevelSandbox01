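; Health actor component that tracks an owner's current and maximum health.
; On begin play it binds to the owner's point damage event, subtracts incoming damage clamped between zero and max health, then fires an OnTakeDamage dispatcher with the new value.
; Setter functions change health and max health directly, and a debug flag draws the current health at the owner's location each tick.
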(event `self.ReceiveBeginPlay`
  (add `Actor.OnTakePointDamage` (`self.GetOwner`) (`|CreateDelegate` :!event `OnTakePointDamage`)))

(event `self.ReceiveTick`
  (params (DeltaSeconds :type "Float (single-precision)"))
  (if (`self.bDebugHealth`)
    (`KismetSystemLibrary.DrawDebugString` (`Actor.K2_GetActorLocation` (`self.GetOwner`)) (`KismetStringLibrary.Conv_DoubleToString` (`self.Health`)) null (struct :`R` 1.0 :`A` 1.0))))

(fn `OnTakePointDamage`
  (params (DamagedActor :type "Actor Object Reference") (Damage :type "Float (single-precision)") (InstigatedBy :type "Controller Object Reference") (HitLocation :type "Vector Structure") (FHitComponent :type "PrimitiveComponent Object Reference") (BoneName :type Name) (ShotFromDirection :type "Vector Structure") (DamageType :type "DamageType Object Reference") (DamageCauser :type "Actor Object Reference"))
  (`self.SetHealth` (`KismetMathLibrary.FClamp` (- (`self.Health`) Damage) 0.0 (`self.MaxHealth`)))
  (`self.OnTakeDamage` (`self.Health`)))

(fn `SetHealth`
  (params (NewHealth :type "Float (double-precision)"))
  (set `self.Health` NewHealth))

(fn `SetMaxHealth`
  (params (NewMaxHealth :type "Float (double-precision)"))
  (set `self.MaxHealth` NewMaxHealth))