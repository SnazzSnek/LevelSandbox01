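; First-person player character with Enhanced Input movement, look, jump, interaction and a hitscan rifle.
; A shared camera line trace drives both the per-tick BP_Interactable check and weapon shots, which use aim or hip spray cones and apply point damage.
; Timers handle held-trigger firing and fire-rate cooldown, while a timeline animates aim FOV.
; Clip, reserve ammo, reload and interact state feed the HUD widget it creates on BeginPlay.
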(event `EnhancedInput|/Game/MyContent/Characters/Player/Inputs/IA_Aim`
  (params (ActionValue :type Boolean) (ElapsedSeconds :type "Float (double-precision)") (TriggeredSeconds :type "Float (double-precision)") (InputAction :type "InputAction Object Reference" :default "/Game/MyContent/Characters/Player/Inputs/IA_Aim.IA_Aim"))
  ;[1 1 1] Aim
  (:`Triggered`
    (if ActionValue
      (`self.TryAim`)
      (else
        (`self.StopAim`)))))

(event `self.ReceiveBeginPlay`
  ;[1 1 1] Begin Play
  ;;[1 1 1] ADD IMC
  (`self.Add Input` "/Game/MyContent/Characters/Player/Inputs/IMC_Locomotion.IMC_Locomotion")
  ;;[1 1 1] Create Player HUD
  (`self.CreatePlayerHUD`)
  (`KismetSystemLibrary.K2_SetTimerDelegate` (`|CreateDelegate` :!event `InteractTrace`))
  (`self.RefreshUI`))

(event `EnhancedInput|/Game/MyContent/Characters/Player/Inputs/IA_Reload`
  (params (ActionValue :type Boolean) (ElapsedSeconds :type "Float (double-precision)") (TriggeredSeconds :type "Float (double-precision)") (InputAction :type "InputAction Object Reference" :default "/Game/MyContent/Characters/Player/Inputs/IA_Reload.IA_Reload"))
  ;[1 1 1] Reload
  (:`Triggered`
    (`self.TryReload`)))

(event `self.ReceiveTick`
  (params (DeltaSeconds :type "Float (single-precision)"))
  ;[1 1 1] Event Tick
  ;[1 1 1] interact trace
  (`self.InteractTrace`))

(event `ZoomtoAim`
  ;[1 1 1] Animate Aim
  (bind (_direction _alpha) (`Timeline|TL_AIM` :!label _label)
    (:`Update`
      (`CameraComponent.SetFieldOfView` (`self.FPSCamera`) (`KismetMathLibrary.Lerp` (`self.StandardZoomAngle`) (`self.AimZoomAngle`) _alpha)))))

(event `EnhancedInput|/Game/MyContent/Characters/Player/Inputs/IA_Movement`
  (params (ActionValue :type "Vector2D Structure") (ElapsedSeconds :type "Float (double-precision)") (TriggeredSeconds :type "Float (double-precision)") (InputAction :type "InputAction Object Reference" :default "/Game/MyContent/Characters/Player/Inputs/IA_Movement.IA_Movement"))
  (bind (_returnvalue_roll _returnvalue_pitch _returnvalue_yaw) (`KismetMathLibrary.BreakRotator` (`self.GetControlRotation`)))
  (bind _returnvalue (`KismetMathLibrary.MakeRotator` 0.0 0.0 _returnvalue_yaw))
  ;[1 1 1] Controls
  (:`Triggered`
    (`|ExecutionSequence`
      (:`then_0`
        ;[1 1 1] Forward Movement
        (`self.AddMovementInput` (`KismetMathLibrary.GetForwardVector` _returnvalue) ActionValue_X))
      (:`then_1`
        ;[1 1 1] Right Movement
        (`self.AddMovementInput` (`KismetMathLibrary.GetRightVector` _returnvalue) ActionValue_Y)))))

(event `ZoomToDefault`
  ;[1 1 1] Animate Aim
  (goto _label :!via `Reverse`))

(event `EnhancedInput|/Game/MyContent/Characters/Player/Inputs/IA_Interact`
  (params (ActionValue :type Boolean) (ElapsedSeconds :type "Float (double-precision)") (TriggeredSeconds :type "Float (double-precision)") (InputAction :type "InputAction Object Reference" :default "/Game/MyContent/Characters/Player/Inputs/IA_Interact.IA_Interact"))
  ;[1 1 1] interact with the interactable
  (:`Triggered`
    (if ActionValue
      (`self.InteractWithInteractable`))))

(event `EnhancedInput|/Game/MyContent/Characters/Player/Inputs/IA_Shoot`
  (params (ActionValue :type Boolean) (ElapsedSeconds :type "Float (double-precision)") (TriggeredSeconds :type "Float (double-precision)") (InputAction :type "InputAction Object Reference" :default "/Game/MyContent/Characters/Player/Inputs/IA_Shoot.IA_Shoot"))
  ;[1 1 1] shooot
  (:`Triggered`
    (if ActionValue
      (`self.StartShooting`)
      (else
        (`self.StopShooting`)))))

(event `EnhancedInput|/Game/MyContent/Characters/Player/Inputs/IA_Camera`
  (params (ActionValue :type "Vector2D Structure") (ElapsedSeconds :type "Float (double-precision)") (TriggeredSeconds :type "Float (double-precision)") (InputAction :type "InputAction Object Reference" :default "/Game/MyContent/Characters/Player/Inputs/IA_Camera.IA_Camera"))
  ;[1 1 1] Controls
  (:`Triggered`
    (`|ExecutionSequence`
      (:`then_0`
        (`self.AddControllerYawInput` ActionValue_X))
      (:`then_1`
        (`self.AddControllerPitchInput` (* ActionValue_Y -1.0))))))

(event `EnhancedInput|/Game/MyContent/Characters/Player/Inputs/IA_Jump`
  (params (ActionValue :type Boolean) (ElapsedSeconds :type "Float (double-precision)") (TriggeredSeconds :type "Float (double-precision)") (InputAction :type "InputAction Object Reference" :default "/Game/MyContent/Characters/Player/Inputs/IA_Jump.IA_Jump"))
  ;[1 1 1] Jumping
  (:`Triggered`
    (if ActionValue
      (`self.Jump`)
      (else
        (`self.StopJumping`)))))

(fn `Add Input`
  (params (MappingContext :type "InputMappingContext Object Reference"))
  ;[1 1 1] adds input to the keyboard
  (`EnhancedInputSubsystemInterface.AddMappingContext` (pcsubsystem `EnhancedInputLocalPlayerSubsystem` (`GameplayStatics.GetPlayerController` 0)) MappingContext 0 (struct)))

(fn `AddAmmo`
  (params (Amount :type Integer))
  (returns (Success :type Boolean))
  (locals (LpreviousAmmo :type Integer))
  (set `local.LpreviousAmmo` (`self.Ammo`))
  (set `self.Ammo` (`KismetMathLibrary.Clamp` (+ (`self.Ammo`) Amount) 0 (`self.Max Ammo`)))
  (`self.UpdateAmmoUI`))

(fn `ClearInteractable`
  ;[1 1 1] clears the interactable from the UI
  (bind _currentinteractable (`self.CurrentInteractable`)
    (:`then`
      (set `self.CurrentInteractable` _currentinteractable)
      (`/Game/MyContent/UI/BP_UI_HUD.SetInteract` (`self.BP_UI_HUD`) false))
    (:`else`)))

(fn `CompleteReload`
  (`self.Reload Ammo`)
  (set `self.bIsReloading` false))

(fn `CoolDownShoot`
  ;[1 1 1] shoot cool down between how many times you can shoot at once
  (set `self.ShootOnCooldown` true)
  (`KismetSystemLibrary.K2_SetTimerDelegate` (`|CreateDelegate` :!event `EndShootCooldown`) (`self.FireRate`)))

(fn `CreatePlayerHUD`
  ;[1 1 1] creates player hud
  (bind _returnvalue (`|CreateWidget` "/Game/MyContent/UI/BP_UI_HUD.BP_UI_HUD_C" (`GameplayStatics.GetPlayerController` 0)))
  (bind _output_get (set `self.BP_UI_HUD` _returnvalue))
  (`UserWidget.AddToPlayerScreen` _output_get 0))

(fn `EndShootCooldown`
  ;[1 1 1] ends the shoot cooldown
  (set `self.ShootOnCooldown` false))

(fn `InteractTrace`
  ;[1 1 1] interact line trace that determines whether or not you are interacting with an interactable
  (bind (_returnvalue _outhit) (`self.LineTraceFromCamera` (`self.InteractDistance`) "TraceTypeQuery3"))
  (if _returnvalue
    (bind _asbp_interactable (cast `/Game/MyContent/Interactables/BP_Interactable` (`.HitActor` (`GameplayStatics.BreakHitResult` _outhit)))
      (:`then`
        (`self.SetCurrentInteractable` _asbp_interactable))
      (:`CastFailed`
        (`self.ClearInteractable`)))
    (else
      (`self.ClearInteractable`))))

(fn `InteractWithInteractable`
  ;[1 1 1] determines whether you are interacting with an object
  (bind _currentinteractable (`self.CurrentInteractable`)
    (:`then`
      (`/Game/MyContent/Interactables/BP_Interactable.Interact` _currentinteractable))
    (:`else`)))

(fn `LineTraceFromCamera`
  (params (Distance :type "Float (double-precision)") (TraceChannel :type "ETraceTypeQuery Enum" :default "TraceTypeQuery1") (DrawDebugType :type "EDrawDebugTrace Enum" :default "None") (SprayAngle :type "Float (single-precision)" :default 3.0))
  (returns (ReturnValue :type Boolean) (OutHit :type "HitResult Structure"))
  (bind _fpscamera (`self.FPSCamera`))
  (bind _returnvalue (`SceneComponent.K2_GetComponentLocation` _fpscamera))
  ;[1 1 1] shoots a line trace from the camera
  (bind (_outhit _returnvalue_2) (`KismetSystemLibrary.LineTraceSingle` :`Start` _returnvalue :`End` (+ _returnvalue (* (`KismetMathLibrary.RandomUnitVectorInConeInDegrees` (`SceneComponent.GetForwardVector` _fpscamera) SprayAngle) Distance)) :`TraceChannel` TraceChannel :`DrawDebugType` DrawDebugType :`DrawTime` 0.5))
  (return _returnvalue_2 _outhit))

(fn `RefreshUI`
  (bind _bp_ui_hud (`self.BP_UI_HUD`)
    (:`then`
      (`/Game/MyContent/UI/BP_UI_HUD.Set Clip` _bp_ui_hud (`self.WeaponClip`))
      (`/Game/MyContent/UI/BP_UI_HUD.SetAmmo` (`self.BP_UI_HUD`) (`self.Ammo`)))
    (:`else`
      (`KismetSystemLibrary.K2_SetTimerDelegate` (`|CreateDelegate` :!event `RefreshUI`) 0.25))))

(fn `Reload Ammo`
  (locals (LreloadAmount :type Integer :default 0))
  (bind _output_get (set `local.LreloadAmount` (`KismetMathLibrary.Clamp` (- (`self.MaxWeaponClip`) (`self.WeaponClip`)) 0 (`self.Ammo`))))
  (set `self.Ammo` (- (`self.Ammo`) _output_get))
  (set `self.WeaponClip` (+ (`self.WeaponClip`) (`local.LreloadAmount`)))
  (`self.UpdateAmmoUI`))

(fn `SetCurrentInteractable`
  (params (CurrentInteractable :type "/Game/MyContent/Interactables/BP_Interactable Object Reference"))
  ;[1 1 1] sets the interactable to be interacted with
  (bind _output_get (set `self.CurrentInteractable` CurrentInteractable))
  (`/Engine/EditorBlueprintResources/StandardMacros.IsValid` _output_get
    (:`Is Valid`
      (`/Game/MyContent/UI/BP_UI_HUD.SetInteract` (`self.BP_UI_HUD`) true))))

(fn `ShootLineTrace`
  (returns (ImpactPoint :type "Vector Structure") (Hit :type Boolean))
  ;[1 1 1] uses a line trace for "shooting"
  (bind (_returnvalue _outhit) (`self.LineTraceFromCamera` (`self.WeaponRange`) "TraceTypeQuery1" "None" (`KismetMathLibrary.SelectFloat` (`self.WeaponAimSprayAngle`) (`self.WeaponHipSprayAngle`) (`self.bIsAiming`))))
  (if _returnvalue
    (bind (_bblockinghit _binitialoverlap _time _distance _location _impactpoint _normal _impactnormal _physmat _hitactor) (`GameplayStatics.BreakHitResult` _outhit))
    (`GameplayStatics.ApplyPointDamage` _hitactor (`self.WeaponDamage`) _normal _outhit null self)
    (return _impactpoint true)
    (else
      (return (0.0 0.0 0.0) false))))

(fn `ShootWeapon`
  (`|ExecutionSequence`
    (:`then_0`
      (bind (_impactpoint _hit) (`self.ShootLineTrace`))
      (if _hit
        (`GameplayStatics.SpawnEmitterAtLocation` "/Game/MilitaryWeapDark/FX/P_Impact_Metal_Small_01.P_Impact_Metal_Small_01" _impactpoint)))
    (:`then_1`
      (`self.UseAmmo`)
      (`AnimInstance.Montage_Play` (`SkeletalMeshComponent.GetAnimInstance` (`self.SKMWeapon`)) "/Game/MilitaryWeapDark/Weapons/Anims/Fire_Rifle_W_Montage.Fire_Rifle_W_Montage" 1.0 "Duration" 0.0 true)
      (`self.CoolDownShoot`))))

(fn `StartReload`
  (params (CooldownTime :type "Float (double-precision)"))
  (set `self.bIsReloading` true)
  (`/Game/MyContent/UI/BP_UI_HUD.PlayReloadTimer` (`self.BP_UI_HUD`) CooldownTime)
  (if (> CooldownTime 0.0)
    (`KismetSystemLibrary.K2_SetTimerDelegate` (`|CreateDelegate` :!event `CompleteReload`) CooldownTime)
    (else
      (`self.CompleteReload`))))

(fn `StartShooting`
  ;[1 1 1] starts shooting when used
  (`KismetSystemLibrary.K2_SetTimerDelegate` (`|CreateDelegate` :!event `TryShoot`) 0.01 true))

(fn `StopAim`
  (if (`self.bIsAiming`)
    (set `self.bIsAiming` false)
    (`self.ZoomToDefault`)))

(fn `StopShooting`
  ;[1 1 1] stops shooting when used
  (`KismetSystemLibrary.K2_ClearTimer` null "TryShoot"))

(fn `TryAim`
  (if (not (`self.bIsAiming`))
    (set `self.bIsAiming` true)
    (`self.ZoomtoAim`)))

(fn `TryReload`
  (if (not (`self.bIsReloading`))
    (set `self.bIsReloading` true)
    (`AnimInstance.Montage_Play` (`SkeletalMeshComponent.GetAnimInstance` (`self.SKMWeapon`)) "/Game/MilitaryWeapDark/Weapons/Anims/Reload_Rifle_Hip_W_Montage.Reload_Rifle_Hip_W_Montage" 1.0 "Duration" 0.0 true)
    (`KismetSystemLibrary.K2_SetTimerDelegate` (`|CreateDelegate` :!event `CompleteReload`))
    (`self.StartReload` 0.0)))

(fn `TryShoot`
  ;[1 1 1] Try shooting function to determine whether you can shoot
  (if (> (`self.WeaponClip`) 0)
    (if (and (not (`self.ShootOnCooldown`)) (not (`self.bIsReloading`)))
      (`self.ShootWeapon`))
    (else
      (`/Game/MyContent/UI/BP_UI_HUD.NeedToReload` (`self.BP_UI_HUD`)))))

(fn `UpdateAmmoUI`
  (`/Game/MyContent/UI/BP_UI_HUD.Set Clip` (`self.BP_UI_HUD`) (`self.WeaponClip`))
  (`/Game/MyContent/UI/BP_UI_HUD.SetAmmo` (`self.BP_UI_HUD`) (`self.Ammo`)))

(fn `UseAmmo`
  ;[1 1 1] uses ammo when shooting
  (`/Engine/EditorBlueprintResources/StandardMacros.DecrementInt` (`self.WeaponClip`)
    (:`  `
      (`self.UpdateAmmoUI`))))

(fn `UserConstructionScript`
  (`parent.UserConstructionScript`)
  (`CameraComponent.SetFieldOfView` (`self.FPSCamera`) (`self.StandardZoomAngle`)))