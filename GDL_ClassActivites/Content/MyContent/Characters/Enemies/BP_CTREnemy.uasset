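; BP_CTREnemy is an enemy character that is tied to an enemy camp and explodes on death.
; Its construction script calls the parent's, then stores the nearest BP_EnemyCamp in the Camp variable.
; When the BP_AC_Health component reports damage leaving health at zero or below, it spawns a rocket-launcher explosion emitter at its location and destroys itself.
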(event `self.BP_AC_Health.OnTakeDamage`
  (params (NewHealth :type "Float (double-precision)"))
  (if (<= NewHealth 0.0)
    (`GameplayStatics.SpawnEmitterAtLocation` "/Game/MilitaryWeapDark/FX/P_RocketLauncher_Explosion_01.P_RocketLauncher_Explosion_01" (`self.K2_GetActorLocation`))
    (`self.K2_DestroyActor`)))

(fn `UserConstructionScript`
  (`parent.UserConstructionScript`)
  (bind _outactors (`GameplayStatics.GetAllActorsOfClass` "/Game/MyContent/Characters/Enemies/BP_EnemyCamp.BP_EnemyCamp_C"))
  (bind _asbp_enemy_camp (cast `/Game/MyContent/Characters/Enemies/BP_EnemyCamp` (`.ReturnValue` (`GameplayStatics.FindNearestActor` (`self.K2_GetActorLocation`) _outactors))))
  (set `self.Camp` _asbp_enemy_camp))